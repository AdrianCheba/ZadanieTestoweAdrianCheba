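; Race car Blueprint that applies the player's chosen paint and race settings and shows driving HUD widgets.
; On BeginPlay it copies max lap time and lap count from BP_GameInstance, runs CustomCar and adds a speedometer widget.
; CustomCar sets the chosen material on body panels, only under a PlayerController.
; Player-controlled mesh hits add a new check-engine widget whenever CurrentDamage is at least 5; damage is not updated here.
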(event `self.ReceiveBeginPlay`
  (bind _asbp_game_instance (cast `/Game/Blueprints/BP_GameInstance` (`GameplayStatics.GetGameInstance`)))
  (set `self.MaxLapTime` (`/Game/Blueprints/BP_GameInstance.MaxLapTime` _asbp_game_instance))
  (bind _asbp_game_instance_2 (cast `/Game/Blueprints/BP_GameInstance` (`GameplayStatics.GetGameInstance`)))
  (set `self.NumberOfLaps` (`/Game/Blueprints/BP_GameInstance.Laps` _asbp_game_instance_2))
  (`self.CustomCar`)
  (bind _returnvalue (`|CreateWidget` "/Game/UI/Speedometer/WB_Speedometer.WB_Speedometer_C"))
  (`UserWidget.AddToViewport` _returnvalue 0))

(event `self.ReceiveTick`
  (params (DeltaSeconds :type "Float (single-precision)")))

(event `self.Mesh.OnComponentHit`
  (params (HitComponent :type "PrimitiveComponent Object Reference") (OtherActor :type "Actor Object Reference") (OtherComp :type "PrimitiveComponent Object Reference") (NormalImpulse :type "Vector Structure") (Hit :type "HitResult Structure (by ref)"))
  (cast `PlayerController` (`self.GetController`))
  (if (>= (`self.CurrentDamage`) 5)
    (bind _returnvalue (`|CreateWidget` "/Game/UI/CheckEngine/WB_CheckEngine.WB_CheckEngine_C"))
    (`UserWidget.AddToViewport` _returnvalue 0)))

(fn `CustomCar`
  (cast `PlayerController` (`self.GetController`))
  (bind _asbp_game_instance (cast `/Game/Blueprints/BP_GameInstance` (`GameplayStatics.GetGameInstance`)))
  (bind _chosenmaterial (`/Game/Blueprints/BP_GameInstance.ChosenMaterial` _asbp_game_instance))
  (`PrimitiveComponent.SetMaterial` (`self.Body`) 0 _chosenmaterial)
  (`PrimitiveComponent.SetMaterial` (`self.WingMirrorRight`) 0 _chosenmaterial)
  (`PrimitiveComponent.SetMaterial` (`self.HoodFront`) 0 _chosenmaterial)
  (`PrimitiveComponent.SetMaterial` (`self.BumperFront`) 0 _chosenmaterial)
  (`PrimitiveComponent.SetMaterial` (`self.BumperRear`) 0 _chosenmaterial)
  (`PrimitiveComponent.SetMaterial` (`self.WingMirrorLeft`) 0 _chosenmaterial)
  (`PrimitiveComponent.SetMaterial` (`self.FenderLeft`) 0 _chosenmaterial)
  (`PrimitiveComponent.SetMaterial` (`self.DoorRight`) 0 _chosenmaterial)
  (`PrimitiveComponent.SetMaterial` (`self.DoorLeft`) 0 _chosenmaterial)
  (`PrimitiveComponent.SetMaterial` (`self.FenderRight`) 0 _chosenmaterial)
  (`PrimitiveComponent.SetMaterial` (`self.SpoilerBack`) 0 _chosenmaterial)
  (`PrimitiveComponent.SetMaterial` (`self.BootRear`) 0 _chosenmaterial))

(fn `UserConstructionScript`)